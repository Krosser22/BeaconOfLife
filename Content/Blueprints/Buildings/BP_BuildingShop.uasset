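; BP_BuildingShop is a shop building that sells food and drink items to characters for money.
; BuyFood and BuyDrink each spawn their item far off-map and disabled to read its BuyPrice.
; If the buyer can afford it, the price is deducted and the item goes into their inventory; otherwise it is destroyed.
; Both return success or failure, and the event graph holds no active logic.
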(fn `BuyDrink`
  (params (CharacterWhoWantsToBuy :type "BeaconOfLife_AI Object Reference"))
  (returns (SuccessfulPurchase :type Boolean))
  (bind _money (`BeaconOfLife_AI.Money` CharacterWhoWantsToBuy))
  (bind _returnvalue (`|SpawnActorFromClass` "/Game/Blueprints/Items/BP_ItemDrink.BP_ItemDrink_C" (`KismetMathLibrary.MakeTransform` (9999.0 9999.0 9999.0)) "AlwaysSpawn" "OverrideRootScale"))
  (set `Item.enabled` false _returnvalue)
  (bind _buyprice (`Item.BuyPrice` _returnvalue))
  (if (>= _money _buyprice)
    (set `BeaconOfLife_AI.Money` (- _money _buyprice) CharacterWhoWantsToBuy)
    (`KismetSystemLibrary.PrintString` (`KismetStringLibrary.Conv_DoubleToString` (`Drink.AmountOfPower` _returnvalue)))
    (`BeaconOfLife_AI.AddDrinkToInventory` CharacterWhoWantsToBuy _returnvalue)
    (return true)
    (else
      ;[1 1 1] The character doesn't have the needed money
      (`self.K2_DestroyActor` _returnvalue)
      (`KismetSystemLibrary.PrintString` "Character has no money")
      (return false))))

(fn `BuyFood`
  (params (CharacterWhoWantsToBuy :type "BeaconOfLife_AI Object Reference"))
  (returns (SuccessfulPurchase :type Boolean))
  (bind _money (`BeaconOfLife_AI.Money` CharacterWhoWantsToBuy))
  (bind _returnvalue (`|SpawnActorFromClass` "/Game/Blueprints/Items/BP_ItemFood.BP_ItemFood_C" (`KismetMathLibrary.MakeTransform` (9999.0 9999.0 9999.0)) "AlwaysSpawn" "OverrideRootScale"))
  (set `Item.enabled` false _returnvalue)
  (bind _buyprice (`Item.BuyPrice` _returnvalue))
  (if (>= _money _buyprice)
    (set `BeaconOfLife_AI.Money` (- _money _buyprice) CharacterWhoWantsToBuy)
    (`BeaconOfLife_AI.AddFoodToInventory` CharacterWhoWantsToBuy _returnvalue)
    (return true)
    (else
      ;[1 1 1] The character doesn't have the needed money
      (`self.K2_DestroyActor` _returnvalue)
      (`KismetSystemLibrary.PrintString` "Character has no money")
      (return false))))

(fn `UserConstructionScript`
  (`parent.UserConstructionScript`))