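; Base Blueprint for buildings, handling overlap tracking before construction and the switch to an abandoned state.
; While the building is not built, begin and end overlap events raise and lower a counter of overlapping buildings and environment actors.
; SetAbandoned adds the building to the first Town Hall's abandoned list and swaps its material to rock, or prints an error if no Town Hall exists.
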(event `self.ReceiveActorBeginOverlap`
  (params (OtherActor :type "Actor Object Reference"))
  (if (not (`self.IsBuilt`))
    (cast `BuildingBase` OtherActor
      (:`then`
        _)
      (:`CastFailed`
        (cast `Environment` OtherActor)))
    (set `self.ObjectsOverlaping` (+ (`self.ObjectsOverlaping`) 1))))

(event `self.ReceiveActorEndOverlap`
  (params (OtherActor :type "Actor Object Reference"))
  (if (not (`self.IsBuilt`))
    (cast `BuildingBase` OtherActor
      (:`then`
        _)
      (:`CastFailed`
        (cast `Environment` OtherActor)))
    (set `self.ObjectsOverlaping` (- (`self.ObjectsOverlaping`) 1))))

(fn `SetAbandoned`
  (bind _outactors (`GameplayStatics.GetAllActorsOfClass` "/Game/Blueprints/Buildings/BP_BuildingTownHall.BP_BuildingTownHall_C"))
  (if (> (`KismetArrayLibrary.Array_Length` _outactors) 0)
    (`KismetArrayLibrary.Array_Add` (`/Game/Blueprints/Buildings/BP_BuildingTownHall.AbandonedBuildings` (`KismetArrayLibrary.Array_Get` _outactors)) self)
    (`PrimitiveComponent.SetMaterial` (`self.Building`) 0 "/Game/StarterContent/Props/Materials/M_Rock.M_Rock")
    (else
      (`KismetSystemLibrary.PrintString` "ERROR: There is not a TownHall" true true (struct :`G` 0.66 :`B` 1.0 :`A` 1.0) 5.0))))

(fn `UserConstructionScript`)