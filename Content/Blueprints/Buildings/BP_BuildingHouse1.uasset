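; BP_BuildingHouse1 is a house building where the owner's family members can sleep.
; Its Sleep function checks the character against BuildingOwner's family, then applies SleepPerFrame scaled by world delta seconds to that character.
; It returns true while the character's Sleep stat is below MaxSleepObtainable, and false at that limit or for non-family.
; Event graph stubs are disabled, and construction only calls the parent.
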(event EventBeginPlay)

(event Collision|EventActorBeginOverlap
  (params (OtherActor :type Actor%20Object%20Reference)))

(event EventTick
  (params (DeltaSeconds :type Float%20%28single-precision%29)))

(fn ConstructionScript
  (|CallParentFunction))

(fn Sleep
  (params (CharacterWhoWantsToSleep :type Beacon%20Of%20Life%20AI%20Object%20Reference))
  (bind _returnvalue (Class|BeaconOfLifeAI|IsFamily (Variables|Default|GetBuildingOwner) CharacterWhoWantsToSleep))
  (if _returnvalue
    (Class|BeaconOfLifeAI|Sleep CharacterWhoWantsToSleep (* (Variables|Default|GetSleepPerFrame) (Utilities|Time|GetWorldDeltaSeconds)))
    (return (< (.sleep (Variables|/Script/BeaconOfLife.BeaconOfLife_AI|GetPhysiologicalStats CharacterWhoWantsToSleep)) (Variables|Default|GetMaxSleepObtainable)))
    (else
      (return false))))