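; Hospital building Blueprint that lets characters pay money to be healed.
; PayHeal deducts the heal cost when the character can afford it, then returns whether the remaining Money still covers that cost.
; GetHeal applies a per-frame heal amount through the character's Heal function and always returns true, with no payment check of its own.
; The event graph is unused, so both functions rely on external callers.
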(fn `GetHeal`
  (params (CharacterWhoWantsToGetHeal :type "BeaconOfLife_AI Object Reference"))
  (returns (SuccessfulHeal :type Boolean))
  (`BeaconOfLife_AI.Heal` CharacterWhoWantsToGetHeal (`self.AmountOfHealPerFrame`))
  (return true))

(fn `PayHeal`
  (params (CharacterWhoWantsToPay :type "BeaconOfLife_AI Object Reference"))
  (returns (SuccessfulPaid :type Boolean))
  (bind _money (`BeaconOfLife_AI.Money` CharacterWhoWantsToPay))
  (bind _amountofmoneytoheal (`self.AmountOfMoneyToHeal`))
  (bind _returnvalue (>= _money _amountofmoneytoheal))
  (if _returnvalue
    (set `BeaconOfLife_AI.Money` (- _money _amountofmoneytoheal) CharacterWhoWantsToPay))
  (return _returnvalue))

(fn `UserConstructionScript`
  (`parent.UserConstructionScript`))