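; Town hall building actor that seeds the town with AI actors and hands out jobs.
; On BeginPlay, it tops up BP_AI actors to at least two, spawning any missing ones at its own transform.
; GetJob pops the first entry of JobList, rebuilding it when empty.
; CreateJobList acts as a shuffle bag holding two of each job type, including none, so assignments stay random but evenly spread.
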(event EventBeginPlay
  (bind _returnvalue (Transformation|GetActorTransform))
  (bind _outactors (Actor|GetAllActorsOfClass "/Game/Blueprints/Characters/BP_AI.BP_AI_C"))
  (Utilities|Casting|CastToBP_GameMode (Game|GetGameMode))
  (if (== (Utilities|Array|Length _outactors) 0)
    (Game|SpawnActorfromClass "/Game/Blueprints/Characters/BP_AI.BP_AI_C" _returnvalue "Undefined" 0 0)
    (Game|SpawnActorfromClass "/Game/Blueprints/Characters/BP_AI.BP_AI_C" _returnvalue "Undefined" 0 0 :!label _label)
    (elif (== (Utilities|Array|Length _outactors) 1)
      (goto _label))))

(event Collision|EventActorBeginOverlap
  (params (OtherActor :type Actor%20Object%20Reference))
  (|CallParentFunction 0))

(event EventTick
  (params (DeltaSeconds :type Float%20%28single-precision%29)))

(fn ConstructionScript
  (|CallParentFunction))

(fn CreateJobList
  (Utilities|Array|Add (Variables|Default|GetJobList) "Job_None")
  (Utilities|Array|Add (Variables|Default|GetJobList) "Job_Cleaner")
  (Utilities|Array|Add (Variables|Default|GetJobList) "Job_Farmer")
  (Utilities|Array|Add (Variables|Default|GetJobList) "Job_Vendor")
  (Utilities|Array|Add (Variables|Default|GetJobList) "Job_Doctor")
  (Utilities|Array|Add (Variables|Default|GetJobList) "Job_FilmWorker")
  (Utilities|Array|Add (Variables|Default|GetJobList) "Job_Chef")
  (Utilities|Array|Add (Variables|Default|GetJobList) "Job_Librarian")
  (Utilities|Array|Add (Variables|Default|GetJobList) "Job_None")
  (Utilities|Array|Add (Variables|Default|GetJobList) "Job_Cleaner")
  (Utilities|Array|Add (Variables|Default|GetJobList) "Job_Farmer")
  (Utilities|Array|Add (Variables|Default|GetJobList) "Job_Vendor")
  (Utilities|Array|Add (Variables|Default|GetJobList) "Job_Doctor")
  (Utilities|Array|Add (Variables|Default|GetJobList) "Job_FilmWorker")
  (Utilities|Array|Add (Variables|Default|GetJobList) "Job_Chef")
  (Utilities|Array|Add (Variables|Default|GetJobList) "Job_Librarian")
  (Utilities|Array|Shuffle (Variables|Default|GetJobList)))

(fn GetJob
  (bind _joblist (Variables|Default|GetJobList))
  (if (> (Utilities|Array|Length (Variables|Default|GetJobList)) 0)
    _
    (else
      (CallFunction|CreateJobList)))
  (bind _output_get (LocalVariables|SetnewJob (Utilities|Array|Get(acopy) _joblist)))
  (Utilities|Array|RemoveIndex _joblist)
  (return _output_get))