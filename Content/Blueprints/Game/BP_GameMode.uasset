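; BP_GameMode is a Game Mode Blueprint that keeps population counters for AI: how many are alive, born and dead.
; AddAI increments the alive and born counts, while RemoveAI decrements the alive count and increments the dead count.
; The event graph and construction script are empty, so the counters change only when something calls these functions or sets the variables directly.
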(fn `AddAI`
  (set `self.AIAlive` (+ (`self.AIAlive`) 1))
  (set `self.AIBorn` (+ (`self.AIBorn`) 1)))

(fn `RemoveAI`
  (set `self.AIAlive` (- (`self.AIAlive`) 1))
  (set `self.AIDead` (+ (`self.AIDead`) 1)))

(fn `UserConstructionScript`)